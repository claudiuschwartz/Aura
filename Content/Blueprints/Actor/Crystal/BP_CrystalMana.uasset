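; BP_CrystalMana is a mana crystal pickup that applies a Gameplay Ability System effect to actors that touch it.
; On sphere overlap it passes the other actor and its duration effect class to ApplyEffectToTarget, marked as the C++ implementation, then destroys itself.
; An unconnected Blueprint alternative applies an instant effect through the target's AbilitySystemComponent, printing messages when the component or effect class is missing.
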(event OnComponentBeginOverlap(Sphere)
  (params (OverlappedComponent :type Primitive%20Component%20Object%20Reference) (OtherActor :type Actor%20Object%20Reference) (OtherComp :type Primitive%20Component%20Object%20Reference) (OtherBodyIndex :type Integer) (bFromSweep :type Boolean) (SweepResult :type Hit%20Result%20Structure%20%28by%20ref%29))
  ;[1 1 1] CPP Implementation
  (Class|AuraEffectActor|ApplyEffecttoTarget OtherActor (Variables|Default|GetDurationGameplayEffectClass))
  (Actor|DestroyActor))

(fn ConstructionScript)